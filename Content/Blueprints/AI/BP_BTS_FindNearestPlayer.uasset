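; Behavior Tree service that finds the nearest living opponent for an AI-controlled pawn.
; Each tick it sets the target tag to Player for pawns tagged Enemy and to Enemy for all others.
; It scans all actors with that tag, skips those reporting dead through an IsDead message, and writes the closest actor and its distance to Blackboard keys.
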(event `self.ReceiveTickAI`
  (params (OwnerController :type "AIController Object Reference") (ControlledPawn :type "Pawn Object Reference") (DeltaSeconds :type "Float (single-precision)"))
  (`self.Set Target Tag` ControlledPawn)
  (`self.Find Nearest Player` ControlledPawn))

(fn `Find Nearest Player`
  (params (ControlledPawn :type "Pawn Object Reference"))
  (locals (`Nearest Actor` :type "Actor Object Reference") (NearestDistance :type "Float (double-precision)"))
  (`/Engine/EditorBlueprintResources/StandardMacros.IsValid` ControlledPawn
    (:`Is Valid`
      (set `local.Nearest Actor` null)
      (set `local.NearestDistance` 9999999.0)
      (bind _outactors (`GameplayStatics.GetAllActorsWithTag` (`self.TargetTag`)))
      (for _array_element _outactors
        (`/Engine/EditorBlueprintResources/StandardMacros.IsValid` _array_element
          (:`Is Valid`
            (bind _returnvalue (message `CombatInterface.IsDead` _array_element))
            (if (not _returnvalue)
              (bind _returnvalue_2 (`Actor.GetDistanceTo` (`local.ControlledPawn`) _array_element))
              (if (< _returnvalue_2 (`local.NearestDistance`))
                (set `local.NearestDistance` _returnvalue_2)
                (set `local.Nearest Actor` _array_element))))))
      (`BTFunctionLibrary.SetBlackboardValueAsObject` (`self.TargetToFollow_Selector`) (`local.Nearest Actor`))
      (`BTFunctionLibrary.SetBlackboardValueAsFloat` (`self.DistanceToTarget_Selector`) (`local.NearestDistance`)))))

(fn `Set Target Tag`
  (params (ControlledPawn :type "Actor Object Reference"))
  (if (`Actor.ActorHasTag` ControlledPawn "Enemy")
    (set `self.TargetTag` "Player")
    (else
      (set `self.TargetTag` "Enemy"))))