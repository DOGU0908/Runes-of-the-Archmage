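; BP_FadeActor is a static mesh actor that can be hidden or shown through its materials' opacity mask.
; The construction script creates a dynamic instance of each mesh material, and BeginPlay assigns the stored instances to the mesh slots by index.
; FadeOut and Fadein call SetOpacityMask, which writes the OpacityMask scalar parameter on every instance at once, switching instantly with no interpolation.
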(event `self.ReceiveBeginPlay`
  (for (_array_element _array_index) (`self.Dynamic Material Instances`)
    (`PrimitiveComponent.SetMaterial` (`self.StaticMesh`) _array_index _array_element)))

(event `/Game/Blueprints/Actor/FadeActor/BI_FadeInterface.FadeOut`
  (`self.SetOpacityMask` 0.0))

(event `/Game/Blueprints/Actor/FadeActor/BI_FadeInterface.FadeIn`
  (`self.SetOpacityMask` 100.0))

(fn `SetOpacityMask`
  (params (OpacityMask :type "Float (double-precision)"))
  (for _array_element (`self.Dynamic Material Instances`)
    (`MaterialInstanceDynamic.SetScalarParameterValue` _array_element "OpacityMask" OpacityMask)))

(fn `UserConstructionScript`
  (for _array_element (`MeshComponent.GetMaterials` (`self.StaticMesh`))
    (bind _returnvalue (`KismetMaterialLibrary.CreateDynamicMaterialInstance` _array_element))
    (`KismetArrayLibrary.Array_AddUnique` (`self.Dynamic Material Instances`) _returnvalue)))