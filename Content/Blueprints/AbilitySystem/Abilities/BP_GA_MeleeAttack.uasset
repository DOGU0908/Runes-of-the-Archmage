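; Gameplay Ability for a melee attack that damages non-friendly live characters near the avatar's combat socket.
; On activation it turns the avatar toward its combat target and plays the combat montage, both through CombatInterface.
; A melee montage gameplay event triggers a radius query around the socket and damage to each hostile found.
; The ability ends after a short delay following the hit, or immediately if the montage is interrupted or cancelled.
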(event `self.K2_ActivateAbility`
  (bind _returnvalue (`self.GetAvatarActorFromActorInfo`))
  (bind _returnvalue_2 (`self.GetAvatarActorFromActorInfo`))
  (bind _returnvalue_3 (message `EnemyInterface.GetCombatTarget` _returnvalue))
  (bind _ascombat_interface (cast `CombatInterface` _returnvalue))
  (`CombatInterface.UpdateFacingTarget` _ascombat_interface (`Actor.K2_GetActorLocation` _returnvalue_3))
  (bind _returnvalue_4 (`CombatInterface.GetCombatMontage` _ascombat_interface))
  (`AbilityTask_PlayMontageAndWait.CreatePlayMontageAndWaitProxy` "None" _returnvalue_4 1.0 "None" false
    (:`then`
      (`AbilityTask_WaitGameplayEvent.WaitGameplayEvent` (struct :`TagName` "Event.Montage.Attack.Melee") null
        (:`EventReceived`
          (bind _returnvalue_5 (message `CombatInterface.GetCombatSocketLocation` _returnvalue_2))
          (bind _outoverlappingactors (`AbilitySystemLibrary.GetLiveCharactersWithinRadius` _returnvalue_2 (`|MakeArray` _returnvalue_2) 45.0 _returnvalue_5))
          (for _array_element _outoverlappingactors
            (if (`AbilitySystemLibrary.IsNotFriendlyUnit` (`self.GetAvatarActorFromActorInfo`) _array_element)
              (`self.CauseDamage` _array_element)))
          (`KismetSystemLibrary.Delay` 1.0))))
    (:`OnInterrupted`
      _)
    (:`OnCancelled`
      _))
  (`self.K2_EndAbility`))