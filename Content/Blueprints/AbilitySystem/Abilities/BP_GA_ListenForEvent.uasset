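; Gameplay ability that listens for gameplay events under the Attributes tag and turns them into attribute-effect applications on its owner.
; On each event it builds a spec from EventBasedEffectClass and walks EventTags to fill the SetByCaller magnitudes.
; The exactly matching tag receives the event's magnitude and every other listed tag is zeroed, then the spec is applied to self.
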(event `self.K2_ActivateAbility`
  (bind _returnvalue (`self.GetAbilitySystemComponentFromActorInfo`))
  (bind (_asynctaskproxy _payload) (`AbilityTask_WaitGameplayEvent.WaitGameplayEvent` (struct :`TagName` "Attributes") null false false)
    (:`EventReceived`
      (set `self.Spec` (`AbilitySystemComponent.MakeOutgoingSpec` _returnvalue (`self.EventBasedEffectClass`) 1.0 (`AbilitySystemComponent.MakeEffectContext` _returnvalue)))
      (for _array_element (`self.EventTags`)
        (bind (_eventtag _instigator _target _optionalobject _optionalobject2 _contexthandle _instigatortags _targettags _eventmagnitude) (break `GameplayEventData` _payload))
        (if (`BlueprintGameplayTagLibrary.MatchesTag` _array_element _eventtag true)
          (`AbilitySystemBlueprintLibrary.AssignTagSetByCallerMagnitude` (`self.Spec`) _eventtag _eventmagnitude)
          (else
            (`AbilitySystemBlueprintLibrary.AssignTagSetByCallerMagnitude` (`self.Spec`) _array_element))))
      (`AbilitySystemComponent.BP_ApplyGameplayEffectSpecToSelf` _returnvalue (`self.Spec`)))))