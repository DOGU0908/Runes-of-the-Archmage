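; Ice gameplay ability that fires a projectile toward the location under the mouse.
; After committing, it takes the cursor's target data, turns the avatar to face that point through CombatInterface, and plays the avatar's combat montage.
; The Event.Montage.Attack gameplay event triggers the projectile spawn once, syncing it to the animation.
; The ability ends when the montage completes, is interrupted or is cancelled, or when commit fails.
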(event `self.K2_ActivateAbility`
  (bind _returnvalue (`self.K2_CommitAbility`))
  (if _returnvalue
    (bind (_asynctaskproxy _datahandle) (`TargetDataUnderMouse.CreateTargetDataUnderMouse`)
      (:`ValidData`
        (set `self.Target Location` (`.Location` (`GameplayStatics.BreakHitResult` (`AbilitySystemBlueprintLibrary.GetHitResultFromTargetData` _datahandle))))
        (bind _ascombat_interface (cast `CombatInterface` (`self.GetAvatarActorFromActorInfo`)))
        (`CombatInterface.UpdateFacingTarget` _ascombat_interface (`self.Target Location`))
        (bind _returnvalue_2 (`CombatInterface.GetCombatMontage` _ascombat_interface))
        (`AbilityTask_PlayMontageAndWait.CreatePlayMontageAndWaitProxy` "None" _returnvalue_2 1.0 "None" false
          (:`then`
            (`AbilityTask_WaitGameplayEvent.WaitGameplayEvent` (struct :`TagName` "Event.Montage.Attack") null true
              (:`EventReceived`
                (`self.SpawnProjectile` (`self.Target Location`)))))
          (:`OnCompleted`
            (`self.K2_EndAbility` :!label _label))
          (:`OnInterrupted`
            (goto _label))
          (:`OnCancelled`
            (goto _label)))))
    (else
      (`self.K2_EndAbility`))))