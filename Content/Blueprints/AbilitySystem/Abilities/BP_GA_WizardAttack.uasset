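; Gameplay ability for a wizard's projectile attack on its current combat target.
; On activation it turns the avatar toward the target through CombatInterface and plays that avatar's combat montage.
; A montage gameplay event triggers the projectile at the target's re-read location, and the ability ends after a short delay.
; Interruption or cancellation ends it immediately, while normal montage completion does not.
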(event `self.K2_ActivateAbility`
  (bind _returnvalue (`self.GetAvatarActorFromActorInfo`))
  (bind _returnvalue_2 (message `EnemyInterface.GetCombatTarget` _returnvalue))
  (bind _ascombat_interface (cast `CombatInterface` _returnvalue))
  (`CombatInterface.UpdateFacingTarget` _ascombat_interface (`Actor.K2_GetActorLocation` _returnvalue_2))
  (bind _returnvalue_3 (`CombatInterface.GetCombatMontage` _ascombat_interface))
  (`AbilityTask_PlayMontageAndWait.CreatePlayMontageAndWaitProxy` "None" _returnvalue_3 1.0 "None" false
    (:`then`
      (`AbilityTask_WaitGameplayEvent.WaitGameplayEvent` (struct :`TagName` "Event.Montage.Attack.Wizard") null true
        (:`EventReceived`
          (bind _returnvalue_4 (message `EnemyInterface.GetCombatTarget` (`self.GetAvatarActorFromActorInfo`)))
          (`self.SpawnProjectile` (`Actor.K2_GetActorLocation` _returnvalue_4))
          (`KismetSystemLibrary.Delay` 2.0))))
    (:`OnInterrupted`
      _)
    (:`OnCancelled`
      _))
  (`self.K2_EndAbility`))